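; Extended UMG button from an icon pack that swaps the icon shown in its Normal, Hovered, Pressed and Disabled states.
; OverrideStateIcon creates a dynamic material from that state's base image, sets its "Icon Texture" parameter, and writes it into the button style, skipping states without a valid image.
; OverrideAllStatesIcon applies one icon to every state, while UpdatePreview does the same with DefaultIcon.
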(event `UpdatePreview`
  (`self.OverrideStateIcon` (`self.DefaultIcon`))
  (`self.OverrideStateIcon` (`self.DefaultIcon`) "NewEnumerator1")
  (`self.OverrideStateIcon` (`self.DefaultIcon`) "NewEnumerator2")
  (`self.OverrideStateIcon` (`self.DefaultIcon`) "NewEnumerator3"))

(fn `OverrideAllStatesIcon`
  (params (Icon :type "Texture2D Object Reference"))
  (`self.OverrideStateIcon` Icon)
  (`self.OverrideStateIcon` Icon "NewEnumerator1")
  (`self.OverrideStateIcon` Icon "NewEnumerator2")
  (`self.OverrideStateIcon` Icon "NewEnumerator3"))

(fn `OverrideStateIcon`
  (params (Icon :type "Texture2D Object Reference") (Style :type "/Game/ExternalContent/CustomizableIconPacks/SharedData/Enumerations/E_ButtonState Enum" :default "NewEnumerator0"))
  (locals (Style_LOCAL :type "ButtonStyle Structure") (Icon_LOCAL :type "Texture2D Object Reference"))
  (set `local.Icon_LOCAL` Icon)
  (set `local.Style_LOCAL` (`self.WidgetStyle`))
  (switch `/Game/ExternalContent/CustomizableIconPacks/SharedData/Enumerations/E_ButtonState` Style
    (:`NewEnumerator0`
      ;[1 1 1] Override NORMAL state image.
      (bind _normalstateimage (`self.NormalStateImage`)
        (:`then`
          (bind _returnvalue (`KismetMaterialLibrary.CreateDynamicMaterialInstance` (`self.GetParent`) _normalstateimage))
          (`MaterialInstanceDynamic.SetTextureParameterValue` _returnvalue "Icon Texture" (`local.Icon_LOCAL`))
          (bind _structout (setmembers `SlateBrush` :`StructRef` (`.Normal` (break `ButtonStyle` (`local.Style_LOCAL`))) :`ResourceObject` _returnvalue))
          (bind _structout_2 (setmembers `ButtonStyle` :`StructRef` (`local.Style_LOCAL`) :`Normal` _structout))
          (bind _output_get (set `local.Style_LOCAL` _structout_2))
          (`self.SetStyle` _output_get))
        (:`else`)))
    (:`NewEnumerator1`
      ;[1 1 1] Override HOVERED state image.
      (bind _hoveredstateimage (`self.HoveredStateImage`)
        (:`then`
          (bind _returnvalue_2 (`KismetMaterialLibrary.CreateDynamicMaterialInstance` (`self.GetParent`) _hoveredstateimage))
          (`MaterialInstanceDynamic.SetTextureParameterValue` _returnvalue_2 "Icon Texture" (`local.Icon_LOCAL`))
          (bind _structout_3 (setmembers `SlateBrush` :`StructRef` (`.Hovered` (break `ButtonStyle` (`local.Style_LOCAL`))) :`ResourceObject` _returnvalue_2))
          (bind _structout_4 (setmembers `ButtonStyle` :`StructRef` (`local.Style_LOCAL`) :`Hovered` _structout_3))
          (bind _output_get_2 (set `local.Style_LOCAL` _structout_4))
          (`self.SetStyle` _output_get_2))
        (:`else`)))
    (:`NewEnumerator2`
      ;[1 1 1] Override PRESSED state image.
      (bind _pressedstateimage (`self.PressedStateImage`)
        (:`then`
          (bind _returnvalue_3 (`KismetMaterialLibrary.CreateDynamicMaterialInstance` (`self.GetParent`) _pressedstateimage))
          (`MaterialInstanceDynamic.SetTextureParameterValue` _returnvalue_3 "Icon Texture" (`local.Icon_LOCAL`))
          (bind _structout_5 (setmembers `SlateBrush` :`StructRef` (`.Pressed` (break `ButtonStyle` (`local.Style_LOCAL`))) :`ResourceObject` _returnvalue_3))
          (bind _structout_6 (setmembers `ButtonStyle` :`StructRef` (`local.Style_LOCAL`) :`Pressed` _structout_5))
          (bind _output_get_3 (set `local.Style_LOCAL` _structout_6))
          (`self.SetStyle` _output_get_3))
        (:`else`)))
    (:`NewEnumerator3`
      ;[1 1 1] Override DISABLED state image.
      (bind _disablestateimage (`self.DisableStateImage`)
        (:`then`
          (bind _returnvalue_4 (`KismetMaterialLibrary.CreateDynamicMaterialInstance` (`self.GetParent`) _disablestateimage))
          (`MaterialInstanceDynamic.SetTextureParameterValue` _returnvalue_4 "Icon Texture" (`local.Icon_LOCAL`))
          (bind _structout_7 (setmembers `SlateBrush` :`StructRef` (`.Disabled` (break `ButtonStyle` (`local.Style_LOCAL`))) :`ResourceObject` _returnvalue_4))
          (bind _structout_8 (setmembers `ButtonStyle` :`StructRef` (`local.Style_LOCAL`) :`Disabled` _structout_7))
          (bind _output_get_4 (set `local.Style_LOCAL` _structout_8))
          (`self.SetStyle` _output_get_4))
        (:`else`)))))