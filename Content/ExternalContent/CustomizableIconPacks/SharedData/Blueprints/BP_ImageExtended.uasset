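; BP_ImageExtended is an image widget from the customizable icon packs that displays an icon texture on a swappable background material.
; SetNewBackgroundMaterial creates a dynamic instance of the background, feeds the custom icon into its "Icon Texture" parameter and sets it as the brush.
; SetNewIcon updates that parameter on the existing instance and reapplies the brush.
; UpdatePreview rebuilds the material from the current background and icon.
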(event `UpdatePreview`
  (`self.SetNewBackgroundMaterial` (`self.CustomBackground`)))

(fn `SetNewBackgroundMaterial`
  (params (NewBackground :type "MaterialInstanceConstant Object Reference"))
  (bind _output_get (set `self.CustomBackground` NewBackground))
  (bind _returnvalue (`KismetMaterialLibrary.CreateDynamicMaterialInstance` (`self.GetParent`) _output_get))
  (bind _output_get_2 (set `self.DynamicMaterialInterface` _returnvalue))
  (`MaterialInstanceDynamic.SetTextureParameterValue` _output_get_2 "Icon Texture" (`self.CustomIcon`))
  (`self.SetBrushFromMaterial` (`self.DynamicMaterialInterface`)))

(fn `SetNewIcon`
  (params (NewIcon :type "Texture2D Object Reference"))
  (set `self.CustomIcon` NewIcon)
  (`MaterialInstanceDynamic.SetTextureParameterValue` (`self.DynamicMaterialInterface`) "Icon Texture" (`self.CustomIcon`))
  (`self.SetBrushFromMaterial` (`self.DynamicMaterialInterface`)))