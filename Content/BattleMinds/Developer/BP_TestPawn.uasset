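; Developer test pawn for trying out universal camera controls and camera travel in BattleMinds.
; It adds the camera mapping context on BeginPlay and routes Enhanced Input to move, rotate and zoom functions, with right movement orbiting the world origin.
; Tick prints spring arm length for debugging.
; The T key only picks and casts a random tile from BP_Tile_Manager, as the camera travel and castle framing experiments are disconnected.
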(event Input|EnhancedActionEvents|EnhancedInputActionIA_MoveForward
  (params (ActionValue :type Float%20%28double-precision%29) (ElapsedSeconds :type Float%20%28double-precision%29) (TriggeredSeconds :type Float%20%28double-precision%29) (InputAction :type Input%20Action%20Object%20Reference :default "/Game/BattleMinds/Developer/IA_MoveForward.IA_MoveForward"))
  (Class|UniversalCamera|MoveForward ActionValue 1.0 false false))

(event Input|EnhancedActionEvents|EnhancedInputActionIA_MoveRight
  (params (ActionValue :type Float%20%28double-precision%29) (ElapsedSeconds :type Float%20%28double-precision%29) (TriggeredSeconds :type Float%20%28double-precision%29) (InputAction :type Input%20Action%20Object%20Reference :default "/Game/BattleMinds/Developer/IA_MoveRight.IA_MoveRight"))
  (Class|UniversalCamera|RotateYawAroundPivot "0, 0, 0" ActionValue 1.0))

(event Input|EnhancedActionEvents|EnhancedInputActionIA_RotateYaw
  (params (ActionValue :type Float%20%28double-precision%29) (ElapsedSeconds :type Float%20%28double-precision%29) (TriggeredSeconds :type Float%20%28double-precision%29) (InputAction :type Input%20Action%20Object%20Reference :default "/Game/BattleMinds/Developer/IA_RotateYaw.IA_RotateYaw"))
  (Class|UniversalCamera|RotateYaw ActionValue 0.5 false))

(event Input|EnhancedActionEvents|EnhancedInputActionIA_RotatePitch
  (params (ActionValue :type Float%20%28double-precision%29) (ElapsedSeconds :type Float%20%28double-precision%29) (TriggeredSeconds :type Float%20%28double-precision%29) (InputAction :type Input%20Action%20Object%20Reference :default "/Game/BattleMinds/Developer/IA_RotatePitch.IA_RotatePitch"))
  (Class|UniversalCamera|RotatePitch ActionValue 1.0 false))

(event Input|EnhancedActionEvents|EnhancedInputActionIA_ZoomIn
  (params (ActionValue :type Float%20%28double-precision%29) (ElapsedSeconds :type Float%20%28double-precision%29) (TriggeredSeconds :type Float%20%28double-precision%29) (InputAction :type Input%20Action%20Object%20Reference :default "/Game/BattleMinds/Developer/IA_ZoomIn.IA_ZoomIn"))
  (Class|UniversalCamera|Zoomin ActionValue 1.0))

(event Input|EnhancedActionEvents|EnhancedInputActionIA_MoveUp
  (params (ActionValue :type Float%20%28double-precision%29) (ElapsedSeconds :type Float%20%28double-precision%29) (TriggeredSeconds :type Float%20%28double-precision%29) (InputAction :type Input%20Action%20Object%20Reference :default "/Game/BattleMinds/Input/IA_MoveUp.IA_MoveUp"))
  (Class|UniversalCamera|MoveUp ActionValue 1.0 false false))

(event EventBeginPlay
  (bind _asplayer_controller (Utilities|Casting|CastToPlayerController (Pawn|GetController)))
  (Utilities|IsValid (PlayerController|LocalPlayerSubsystems|GetEnhancedInputLocalPlayerSubsystem _asplayer_controller)
    (:Is%20Valid
      (Input|AddMappingContext (PlayerController|LocalPlayerSubsystems|GetEnhancedInputLocalPlayerSubsystem _asplayer_controller) "/Game/BattleMinds/Developer/IMC_UniversalCamera.IMC_UniversalCamera" 0 "(bIgnoreAllPressedKeysUntilRelease=True,bForceImmediately=False,bNotifyUserSettings=False)"))))

(event EventTick
  (params (DeltaSeconds :type Float%20%28single-precision%29))
  (Development|PrintString (Utilities|String|ToString(Float) (Variables|/Script/Engine.SpringArmComponent|GetTargetArmLength (Variables|Default|GetSpringArmComponent))) true true "(R=0.000000,G=0.660000,B=1.000000,A=1.000000)" DeltaSeconds))

(event Input|KeyboardEvents|DebugKeyT
  (params (Key :type Key%20Structure :default "None") (ActionValue :type Input%20Action%20Value%20Structure))
  (:Pressed
    (bind _returnvalue (Actor|GetActorOfClass "/Game/BattleMinds/Core/Tiles/BP_Tile_Manager.BP_Tile_Manager_C"))
    (bind _keys (Utilities|Map|Keys (Variables|/Script/BattleMinds.BM_TileManager|GetTiles _returnvalue)))
    (bind _output_get (Variables|Default|SetTilexAxial (.OutItem (Utilities|Array|Random _keys))))
    (Utilities|Casting|CastToBP_TileBase (.Value (Utilities|Map|Find (Variables|/Script/BattleMinds.BM_TileManager|GetTiles _returnvalue) _output_get)))))

(fn ConstructionScript)