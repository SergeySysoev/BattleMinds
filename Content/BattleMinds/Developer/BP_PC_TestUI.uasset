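; BP_PC_TestUI is a developer test player controller for previewing UI widgets in isolation.
; On BeginPlay it shows a WBP_TestWidgetCreator selector and keeps a reference to it.
; CreateWidgetAndAddToViewport hides the selector and displays a widget of the given class as the tested widget.
; A debug P key press removes the tested widget and brings the selector back.
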(event Custom|CreateWidgetAndAddToViewport
  (params (Class :type User%20Widget%20Class%20Reference))
  (bind _widgetselector (Variables|Default|GetWidgetSelector)
    (:then
      (Widget|RemovefromParent _widgetselector)
      (bind _returnvalue (UserInterface|CreateWidget Class self))
      (UserInterface|Viewport|AddtoViewport _returnvalue 0)
      (Variables|Default|SetTestedWidget _returnvalue))
    (:else)))

(event EventBeginPlay
  (bind _returnvalue (UserInterface|CreateWidget "/Game/BattleMinds/Developer/WBP_TestWidgetCreator.WBP_TestWidgetCreator_C" self))
  (UserInterface|Viewport|AddtoViewport _returnvalue 0)
  (Variables|Default|SetWidgetSelector _returnvalue))

(event Input|KeyboardEvents|DebugKeyP
  (params (Key :type Key%20Structure :default "None") (ActionValue :type Input%20Action%20Value%20Structure))
  (:Pressed
    (bind _testedwidget (Variables|Default|GetTestedWidget)
      (:then
        (Widget|RemovefromParent _testedwidget)
        (Variables|Default|SetTestedWidget 0)
        (UserInterface|Viewport|AddtoViewport (Variables|Default|GetWidgetSelector) 0))
      (:else))))

(fn ConstructionScript)