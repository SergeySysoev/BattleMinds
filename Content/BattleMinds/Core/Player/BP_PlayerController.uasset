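; Player controller for BattleMinds, a turn-based tile and question game, linking player input, game state updates and the HUD.
; The local controller creates the player info HUD; left-click traces under the cursor and submits unattacked tiles through an SC call.
; Prefixed SC, MC and CC calls relay question requests, turn nickname, timer and round updates to the HUD or server.
; Answered questions are forwarded to the player state.
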(event `self.ReceiveBeginPlay`
  (if (`self.IsLocalPlayerController`)
    (bind _returnvalue (`|CreateWidget` "/Game/BattleMinds/Core/UI/WBP_PlayerInfo.WBP_PlayerInfo_C" self))
    (bind _output_get (set `self.PlayerHUD` _returnvalue))
    (`UserWidget.AddToViewport` _returnvalue 0)
    (`UserWidget.AddToViewport` _output_get 0)))

(event `Key|LeftMouseButton`
  (params (Key :type "Key Structure"))
  (:`Pressed`
    (bind _asbm_tile_base (cast `BM_TileBase` (`.HitActor` (`GameplayStatics.BreakHitResult` (`self.GetHitResultUnderCursorForObjects` (`|MakeArray` "ObjectTypeQuery7" :!type "EObjectTypeQuery Enum"))))))
    (if (not (`BM_TileBase.bIsAttacked` _asbm_tile_base))
      (`self.SC_TryClickTheTile` _asbm_tile_base))))

(event `self.OpenQuestion`
  (`self.SC_RequestToOpenQuestion`))

(event `self.UpdateCurrentPlayerNickname`
  (params (CurrentPlayerNickname :type String))
  (`self.MC_UpdateCurrentPlayerNickname` CurrentPlayerNickname))

(event `self.UpdateTurnTimer`
  (params (GameRound :type "EGameRound Enum" :default "ChooseCastle"))
  (`self.CC_UpdateTurnTimer` GameRound))

(event `MC_UpdateCurrentPlayerNickname`
  (params (Nickname :type String))
  (`/Game/BattleMinds/Core/UI/WBP_PlayerInfo.UpdatePlayersTurn` (`self.PlayerHUD`) Nickname))

(event `self.ResetTurnTimer`
  (params (GameRound :type "EGameRound Enum" :default "ChooseCastle"))
  (`self.CC_ResetTurnTimer` GameRound))

(event `CC_UpdateTurnTimer`
  (params (GameRound :type "EGameRound Enum" :default "ChooseCastle"))
  (bind _playerhud (`self.PlayerHUD`))
  (`BM_UWTurnTimer.UpdateTimer` (`/Game/BattleMinds/Core/UI/WBP_PlayerInfo.WBP_TurnTimer` _playerhud))
  (`/Game/BattleMinds/Core/UI/WBP_GameRoundIndicator.SetRoundIndicator` (`/Game/BattleMinds/Core/UI/WBP_PlayerInfo.WBP_GameRoundIndicator` _playerhud) GameRound))

(event `CC_ResetTurnTimer`
  (params (GameRound :type "EGameRound Enum" :default "ChooseCastle"))
  (bind _playerhud (`self.PlayerHUD`))
  (`BM_UWTurnTimer.ResetTimer` (`/Game/BattleMinds/Core/UI/WBP_PlayerInfo.WBP_TurnTimer` _playerhud))
  (`/Game/BattleMinds/Core/UI/WBP_GameRoundIndicator.SetRoundIndicator` (`/Game/BattleMinds/Core/UI/WBP_PlayerInfo.WBP_GameRoundIndicator` _playerhud) GameRound))

(event `SC_AddAnsweredQuestion`
  (params (Question :type "Question Structure"))
  (bind _asbp_player_state (cast `/Game/BattleMinds/Core/Player/BP_PlayerState` (`self.PlayerState`)))
  (`/Game/BattleMinds/Core/Player/BP_PlayerState.SC_AddAnsweredQuestion` _asbp_player_state Question))

(fn `UserConstructionScript`)