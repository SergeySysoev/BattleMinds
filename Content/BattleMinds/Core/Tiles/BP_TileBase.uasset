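; Base actor for a BattleMinds board tile, placed by axial coordinates and handling the tile's visual feedback.
; Timelines drive dynamic-material color changes, raise castle and banner meshes, and zoom the spring-arm camera on damage, firing completion callbacks.
; Castle damage attaches a Niagara explosion to the HP-selected tower or castle, then swaps its mesh, with an editor test variant.
; MC_ events apply material changes and update the points widget.
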(event `self.ReceiveBeginPlay`
  (`PrimitiveComponent.SetCastShadow` (`self.PointsWidget`) false))

(event `UpdateStartingPosition`
  (bind _location (`/Game/ExternalContent/Hex_Grid_Toolkit/BluePrints/Hex_Logic/BPFL_Hex_Logic.AxialToLocationWithStartingPoint` (`self.Axial`) (`self.Starting Point`)))
  (`self.K2_SetActorTransform` (`KismetMathLibrary.MakeTransform` _location)))

(event `self.SwitchTileMeshMaterialColor`
  (`self.MC_TileMaterialChange`))

(event `MC_TileMaterialChange`
  (bind (_direction _tilematerialblend _bannerdissolve) (`Timeline|MeshColorChangeTimeline` :!via `PlayFromStart`)
    (:`Update`
      (bind _returnvalue (`PrimitiveComponent.CreateDynamicMaterialInstance` (`self.TileMesh`) 0 (`self.TileMeshMaterial`) "None"))
      (`MaterialInstanceDynamic.SetScalarParameterValue` _returnvalue "Appearance" _tilematerialblend)
      (`MaterialInstanceDynamic.SetScalarParameterValue` _returnvalue "BlendAlpha" _tilematerialblend))
    (:`Finished`
      (`self.OnTileMaterialSwitched`))))

(event `self.SpawnCastleMesh`
  (bind _castlemesh (`self.CastleMesh`))
  (bind (_returnvalue_x _returnvalue_y _returnvalue_z) (`KismetMathLibrary.BreakVector` (`SceneComponent.K2_GetComponentLocation` (`self.CastleMesh`))))
  (bind (_returnvalue_x_2 _returnvalue_y_2) (`KismetMathLibrary.BreakVector` (`SceneComponent.K2_GetComponentLocation` _castlemesh)))
  (bind (_returnvalue_x_3 _returnvalue_y_3 _returnvalue_z_2) (`KismetMathLibrary.BreakVector` (`SceneComponent.K2_GetComponentLocation` (`self.CastleEndLocation`))))
  ;[1 1 1] Spawn Meshes
  (set `self.OriginalCastleZLocation` _returnvalue_z)
  (bind (_direction _scalez _locationz _castlelocationz _castlelocationalpha) (`Timeline|TileScaleAndZChange` :!via `PlayFromStart`)
    (:`Update`
      (`SceneComponent.K2_SetWorldLocation` _castlemesh (`KismetMathLibrary.MakeVector` _returnvalue_x_2 _returnvalue_y_2 (`KismetMathLibrary.Lerp` (`self.OriginalCastleZLocation`) _returnvalue_z_2 _castlelocationalpha)) false false))
    (:`Finished`
      (`parent.SpawnCastleMesh`)
      (`self.OnCastleMeshSpawned`))))

(event `self.SetPointsWidgetValue`
  (params (Points :type Integer))
  ;[1 0.8629 0] Points Widget
  (`self.MC_SetPoints` Points))

(event `self.PlayTileDamageAnimation`
  ;[1 1 1] Tile Damage
  (set `SpringArmComponent.TargetArmLength` (`self.BaseSpringArmSocketOffset`) (`self.TileSpringArm`))
  (switch `ETileStatus` (`self.CachedStatus`)
    (:`Controlled`
      (bind (_direction _camerazoom) (`Timeline|CameraZoom` :!via `PlayFromStart`)
        (:`Update`
          ;;[0 0 0] DEPRECATED
          (set `SpringArmComponent.TargetArmLength` _camerazoom (`self.TileSpringArm`)))))
    (:`Castle`
      (`NiagaraFunctionLibrary.SpawnSystemAttached` "/Game/ExternalContent/Vefects/Anime_VFX/Shared/Skills/NS_ExplosionGround.NS_ExplosionGround" (select `int` (`self.TileHP`) :`0` (`self.CastleMesh`) :`1` (`self.SecondTowerMesh`) :`2` (`self.FirstTowerMesh`) :!type "SceneComponent Object Reference") "None" (0.0 0.0 0.0) (struct) "KeepRelativeOffset")
      (bind (_direction_2 _damagepercent _camerazoom_2) (`Timeline|TowerDamageTimeline` :!via `PlayFromStart`)
        (:`Update`
          (set `SpringArmComponent.TargetArmLength` _camerazoom_2 (`self.TileSpringArm`)))
        (:`Finished`
          (`StaticMeshComponent.SetStaticMesh` (select `int` (`self.TileHP`) :`0` (`self.CastleMesh`) :`1` (`self.SecondTowerMesh`) :`2` (`self.FirstTowerMesh`)) (select `int` (`self.TileHP`) :`0` "/Game/ExternalContent/Toony_Tiny_RTS_Set_UE5/Meshes/Buildings/Construction/SM_Castle_1.SM_Castle_1" :`1` "/Game/ExternalContent/Toony_Tiny_RTS_Set_UE5/Meshes/Buildings/Construction/SM_Tower_C_0.SM_Tower_C_0" :`2` "/Game/ExternalContent/Toony_Tiny_RTS_Set_UE5/Meshes/Buildings/Construction/SM_Tower_C_0.SM_Tower_C_0" :!type "StaticMesh Object Reference"))
          (`self.OnCastleTowerDamaged`))))))

(event `MC_SetPoints`
  (params (Points :type Integer))
  ;[1 0.8629 0] Points Widget
  (bind _aswbp_tile_points (cast `/Game/BattleMinds/UI/Tiles/WBP_TilePoints` (`WidgetComponent.GetWidget` (`self.PointsWidget`))))
  (`/Game/BattleMinds/UI/Tiles/WBP_TilePoints.SetPoints` _aswbp_tile_points Points 0.0))

(event `self.SpawnBannerMesh`
  (bind _bannermesh (`self.BannerMesh`))
  (bind (_returnvalue_x _returnvalue_y _returnvalue_z) (`KismetMathLibrary.BreakVector` (`SceneComponent.K2_GetComponentLocation` (`self.CastleEndLocation`))))
  (bind (_returnvalue_x_2 _returnvalue_y_2) (`KismetMathLibrary.BreakVector` (`SceneComponent.K2_GetComponentLocation` _bannermesh)))
  (bind (_returnvalue_x_3 _returnvalue_y_3 _returnvalue_z_2) (`KismetMathLibrary.BreakVector` (`SceneComponent.K2_GetComponentLocation` (`self.BannerMesh`))))
  ;[1 1 1] Spawn Meshes
  (set `self.BannerOriginalZLocation` _returnvalue_z_2)
  (bind (_direction _interpalpha) (`Timeline|SpawnBannerTimeline` :!via `PlayFromStart`)
    (:`Update`
      (`SceneComponent.K2_SetWorldLocation` _bannermesh (`KismetMathLibrary.MakeVector` _returnvalue_x_2 _returnvalue_y_2 (`KismetMathLibrary.Lerp` (`self.BannerOriginalZLocation`) _returnvalue_z _interpalpha)) false false))
    (:`Finished`
      (`parent.SpawnBannerMesh`)
      (`self.OnBannerMeshSpawned`))))

(event `EditorTileDamageAnimation`
  (bind _testhp (`self.TestHP`))
  ;[1 1 1] Tile Damage
  (set `SpringArmComponent.TargetArmLength` (`self.BaseSpringArmSocketOffset`) (`self.TileSpringArm`))
  (`NiagaraFunctionLibrary.SpawnSystemAttached` "/Game/ExternalContent/Vefects/Anime_VFX/Shared/Skills/NS_ExplosionGround.NS_ExplosionGround" (select `int` (`self.TestHP`) :`0` (`self.CastleMesh`) :`1` (`self.SecondTowerMesh`) :`2` (`self.FirstTowerMesh`) :!type "SceneComponent Object Reference") "None" (0.0 0.0 0.0) (struct) "KeepRelativeOffset")
  (bind (_direction _damagepercent _camerazoom) (`Timeline|Timeline_0` :!via `PlayFromStart`)
    (:`Update`
      (set `SpringArmComponent.TargetArmLength` _camerazoom (`self.TileSpringArm`)))
    (:`Finished`
      (`StaticMeshComponent.SetStaticMesh` (select `int` _testhp :`0` (`self.CastleMesh`) :`1` (`self.SecondTowerMesh`) :`2` (`self.FirstTowerMesh`)) (select `int` _testhp :`0` "/Game/ExternalContent/Toony_Tiny_RTS_Set_UE5/Meshes/Buildings/Construction/SM_Castle_1.SM_Castle_1" :`1` "/Game/ExternalContent/Toony_Tiny_RTS_Set_UE5/Meshes/Buildings/Construction/SM_Tower_C_0.SM_Tower_C_0" :`2` "/Game/ExternalContent/Toony_Tiny_RTS_Set_UE5/Meshes/Buildings/Construction/SM_Tower_C_0.SM_Tower_C_0" :!type "StaticMesh Object Reference")))))

(fn `UserConstructionScript`)