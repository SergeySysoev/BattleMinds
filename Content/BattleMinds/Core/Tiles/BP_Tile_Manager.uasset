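; BP_Tile_Manager builds and manages the BattleMinds hex territory map.
; GenerateMap spawns BP_TileBase actors into an axial-keyed Tiles map, which status and owner queries scan.
; Hex shape operations derive candidates for castles (map border, spaced from owned tiles), expansion (free neighbours, else any unowned) and attack (territory outline).
; AutoAssignTerritory randomly assigns these round-robin via SCSetTileOwner, with a timed debug variant; toolkit samples and glossary remain unwired.
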(event `AutoAssign`
  ;[0 0 0] DEBUG AUTOASSIGN TILES
  (bind _returnvalue (`KismetSystemLibrary.K2_SetTimerDelegate` (delegate `SetCastle`) 0.5 true))
  (set `self.DEBUG_SetCastleTimer` _returnvalue))

(event `SetCastle`
  ;[0 0 0] DEBUG AUTOASSIGN TILES
  (bind _returnvalue (`self.GetTilesAvailableForCastle`))
  (set `self.DisplayShape` _returnvalue)
  (`self.SC_SetTileOwner` (`KismetArrayLibrary.Array_Random` _returnvalue) "Castle" (`self.CurrentPlayer`) (cast `EColor` (+ (`KismetMathLibrary.Conv_IntToByte` (`self.CurrentPlayer`)) 1)))
  (bind _result (`/Engine/EditorBlueprintResources/StandardMacros.IncrementInt` (`self.CurrentPlayer`))
    (:`  `
      (if (>= _result 3)
        (`KismetSystemLibrary.K2_ClearAndInvalidateTimerHandle` (`self.DEBUG_SetCastleTimer`))
        (bind _shape (`self.Find Tiles Of Status` (`|MakeArray` "NotOwned" :!type "ETileStatus Enum")))
        (set `self.TileNum` (`KismetArrayLibrary.Array_Length` _shape))
        (bind _returnvalue_2 (`KismetSystemLibrary.K2_SetTimerDelegate` (delegate `SetTile`) 0.5 true))
        (set `self.DEBUG_SetTile` _returnvalue_2)))))

(event `SetTile`
  ;[0 0 0] DEBUG AUTOASSIGN TILES
  (if (< (`self.DEBUG_Counter`) (`self.TileNum`))
    (bind _output_get (set `self.CurrentPlayer` (select `bool` (>= (`self.CurrentPlayer`) 3) :`false` (`self.CurrentPlayer`))))
    (bind _returnvalue (`self.GetTilesAvailableForExpansion` _output_get))
    (set `self.DisplayShape` _returnvalue)
    (`self.SC_SetTileOwner` (`KismetArrayLibrary.Array_Random` _returnvalue) "Controlled" (`self.CurrentPlayer`) (cast `EColor` (+ (`KismetMathLibrary.Conv_IntToByte` (`self.CurrentPlayer`)) 1)))
    (`/Engine/EditorBlueprintResources/StandardMacros.IncrementInt` (`self.CurrentPlayer`)
      (:`  `
        (`/Engine/EditorBlueprintResources/StandardMacros.IncrementInt` (`self.DEBUG_Counter`))))
    (else
      (`KismetSystemLibrary.K2_ClearAndInvalidateTimerHandle` (`self.DEBUG_SetTile`)))))

(event `self.ReceiveBeginPlay`
  (`parent.ReceiveBeginPlay`))

(event `HexSelectedUpdate`)

(event `self.ReceiveTick`
  (params (DeltaSeconds :type "Float (single-precision)")))

(event `HexHoverUpdate`)

(fn `AutoAssignTerritory`
  (params (bAssignCastles :type Boolean) (PlayerColors :type "Map of Integer to EColor Enum (by ref)"))
  (locals (NumberOfPlayers :type Integer) (CurrentPlayerCounter :type Integer))
  (set `local.NumberOfPlayers` (`BlueprintMapLibrary.Map_Length` PlayerColors))
  (`|ExecutionSequence`
    (:`then_0`
      (if (`local.bAssignCastles`)
        (bind _keys (`BlueprintMapLibrary.Map_Keys` (`local.PlayerColors`)))
        (for _array_element _keys
          (bind _returnvalue (`self.GetTilesAvailableForCastle`))
          (`self.SC_SetTileOwner` (`KismetArrayLibrary.Array_Random` _returnvalue) "Castle" _array_element (`BlueprintMapLibrary.Map_Find` (`local.PlayerColors`) _array_element)))))
    (:`then_1`
      (for _ (range (+ (- (`BlueprintMapLibrary.Map_Length` (`self.Tiles`)) (`local.NumberOfPlayers`)) 1))
        (set `local.CurrentPlayerCounter` (select `bool` (>= (`local.CurrentPlayerCounter`) (`local.NumberOfPlayers`)) :`false` (`local.CurrentPlayerCounter`)))
        (bind _keys_2 (`BlueprintMapLibrary.Map_Keys` (`local.PlayerColors`)))
        (bind _output (`|GetArrayItem` _keys_2 (`local.CurrentPlayerCounter`)))
        (bind _returnvalue_2 (`self.GetTilesAvailableForExpansion` _output))
        (`self.SC_SetTileOwner` (`KismetArrayLibrary.Array_Random` _returnvalue_2) "Controlled" _output (`BlueprintMapLibrary.Map_Find` (`local.PlayerColors`) (`local.CurrentPlayerCounter`)))
        (`/Engine/EditorBlueprintResources/StandardMacros.IncrementInt` (`local.CurrentPlayerCounter`))))))

(fn `Find Tiles Of Status`
  (params (TileStatus :type "Array of ETileStatus Enum"))
  (returns (Shape :type "Array of IntPoint Structure"))
  (locals (ShapeLocal :type "Array of IntPoint Structure"))
  (bind _tiles (`self.Tiles`))
  (bind _keys (`BlueprintMapLibrary.Map_Keys` _tiles))
  (for _array_element _keys
    (if (`KismetArrayLibrary.Array_Contains` TileStatus (`BM_TileBase.Status` (`BlueprintMapLibrary.Map_Find` _tiles _array_element)))
      (`KismetArrayLibrary.Array_Add` (`local.ShapeLocal`) _array_element)))
  (return (`local.ShapeLocal`)))

(fn `FindTilesOfPlayer`
  (params (PlayerID :type Integer))
  (returns (Shape :type "Array of IntPoint Structure"))
  (locals (ShapeLocal :type "Array of IntPoint Structure"))
  (bind _tiles (`self.Tiles`))
  (bind _keys (`BlueprintMapLibrary.Map_Keys` _tiles))
  (for _array_element _keys
    (if (== (`BM_TileBase.OwnerPlayerID` (`BlueprintMapLibrary.Map_Find` _tiles _array_element)) (`local.PlayerID`))
      (`KismetArrayLibrary.Array_Add` (`local.ShapeLocal`) _array_element)))
  (return (`local.ShapeLocal`)))

(fn `GenerateMap`
  (params (NumberOfPlayers :type Integer))
  (bind _shapeout (`/Game/ExternalContent/Hex_Grid_Toolkit/BluePrints/Hex_Logic/BPFL_Hex_Logic.getShape` "NewEnumerator0" (struct) (make `IntPoint` NumberOfPlayers 5)))
  (for _array_element _shapeout
    (`self.spawnTile` _array_element))
  (`parent.GenerateMap` NumberOfPlayers))

(fn `Get Tile Status`
  (params (Axial :type "IntPoint Structure (by ref)"))
  (returns (Status :type "ETileStatus Enum"))
  (bind _value (`BlueprintMapLibrary.Map_Find` (`self.Tiles`) Axial))
  (`/Engine/EditorBlueprintResources/StandardMacros.IsValid` _value
    (:`Is Valid`
      (return (`BM_TileBase.Status` _value)))))

(fn `GetTilesAvailableForAttack`
  (params (PlayerID :type Integer))
  (returns (ReturnValue :type "Array of IntPoint Structure"))
  (locals (PlayerTerritory :type "Array of IntPoint Structure") (AvailableNeighbors :type "Set of IntPoint Structure") (PossibleTiles :type "Array of IntPoint Structure") (ControlledTiles :type "Array of IntPoint Structure"))
  (`|ExecutionSequence`
    (:`then_0`
      (bind _shape (`self.FindTilesOfPlayer` (`local.PlayerID`)))
      (set `local.PlayerTerritory` _shape)
      (bind _shape_2 (`self.Find Tiles Of Status` (`|MakeArray` "Controlled" "Castle" "Attacked" :!type "ETileStatus Enum")))
      (set `local.ControlledTiles` _shape_2))
    (:`then_1`
      (bind _border (`/Game/ExternalContent/Hex_Grid_Toolkit/BluePrints/Hex_Logic/BPFL_Hex_Logic.getShapeBorder` (`local.PlayerTerritory`) true))
      (`BlueprintSetLibrary.Set_AddItems` (`local.AvailableNeighbors`) _border))
    (:`then_2`
      (bind _result (`BlueprintSetLibrary.Set_ToArray` (`local.AvailableNeighbors`)))
      (set `local.PossibleTiles` _result)
      (return (`local.PossibleTiles`)))))

(fn `GetTilesAvailableForCastle`
  (returns (ReturnValue :type "Array of IntPoint Structure"))
  (locals (ControlledTiles :type "Array of IntPoint Structure") (MapBorder :type "Array of IntPoint Structure") (PossibleTiles :type "Array of IntPoint Structure") (PossibleForCastleTiles :type "Array of IntPoint Structure") (PossibleTilesSet :type "Set of IntPoint Structure"))
  (`|ExecutionSequence`
    (:`then_0`
      (bind _shape (`self.Find Tiles Of Status` (`|MakeArray` "Controlled" "Castle" :!type "ETileStatus Enum")))
      (set `local.ControlledTiles` _shape)
      (bind _keys (`BlueprintMapLibrary.Map_Keys` (`self.Tiles`)))
      (bind _border (`/Game/ExternalContent/Hex_Grid_Toolkit/BluePrints/Hex_Logic/BPFL_Hex_Logic.getShapeBorder` _keys))
      (set `local.MapBorder` _border))
    (:`then_1`
      (bind _difference (`/Game/ExternalContent/Hex_Grid_Toolkit/BluePrints/Hex_Logic/BPFL_Hex_Logic.Get Shapes Symmetric Difference` (`local.MapBorder`) (`local.ControlledTiles`)))
      (set `local.PossibleTiles` _difference)
      (for _array_element (`local.ControlledTiles`)
        (bind _shape_2 (`/Game/ExternalContent/Hex_Grid_Toolkit/BluePrints/Hex_Logic/BPFL_Hex_Logic.Get Hexes In Radius And Shape` _array_element 2 (`local.PossibleTiles`)))
        (`BlueprintSetLibrary.Set_AddItems` (`local.PossibleTilesSet`) _shape_2)
        (`BlueprintSetLibrary.Set_Add` (`local.PossibleTilesSet`) _array_element))
      (bind _result (`BlueprintSetLibrary.Set_ToArray` (`local.PossibleTilesSet`)))
      (bind _keys_2 (`BlueprintMapLibrary.Map_Keys` (`self.Tiles`)))
      (bind _border_2 (`/Game/ExternalContent/Hex_Grid_Toolkit/BluePrints/Hex_Logic/BPFL_Hex_Logic.getShapeBorder` _keys_2))
      (bind _difference_2 (`/Game/ExternalContent/Hex_Grid_Toolkit/BluePrints/Hex_Logic/BPFL_Hex_Logic.Get Shapes Symmetric Difference` _border_2 _result))
      (set `self.DisplayShape` _difference_2)
      (set `local.PossibleForCastleTiles` _difference_2))
    (:`then_2`
      (return (`local.PossibleForCastleTiles`)))))

(fn `GetTilesAvailableForExpansion`
  (params (PlayerID :type Integer))
  (returns (ReturnValue :type "Array of IntPoint Structure"))
  (locals (PossibleTiles :type "Array of IntPoint Structure") (PlayerTerritory :type "Array of IntPoint Structure") (AvailableNeighbors :type "Set of IntPoint Structure") (ControlledTiles :type "Array of IntPoint Structure"))
  (`|ExecutionSequence`
    (:`then_0`
      (bind _shape (`self.FindTilesOfPlayer` (`local.PlayerID`)))
      (set `local.PlayerTerritory` _shape)
      (bind _shape_2 (`self.Find Tiles Of Status` (`|MakeArray` "Controlled" "Castle" "Attacked" :!type "ETileStatus Enum")))
      (set `local.ControlledTiles` _shape_2))
    (:`then_1`
      (for _array_element (`local.PlayerTerritory`)
        (bind _keys (`BlueprintMapLibrary.Map_Keys` (`self.Tiles`)))
        (bind _axials (`/Game/ExternalContent/Hex_Grid_Toolkit/BluePrints/Hex_Logic/BPFL_Hex_Logic.getNeighboursInShape` _array_element _keys))
        (bind _resultingshape (`/Game/ExternalContent/Hex_Grid_Toolkit/BluePrints/Hex_Logic/BPFL_Hex_Logic.SubstractShapes` _axials (`local.ControlledTiles`)))
        (`BlueprintSetLibrary.Set_AddItems` (`local.AvailableNeighbors`) _resultingshape)))
    (:`then_2`
      (if (`BlueprintSetLibrary.Set_IsEmpty` (`local.AvailableNeighbors`))
        (bind _shape_3 (`self.Find Tiles Of Status` (`|MakeArray` "NotOwned" :!type "ETileStatus Enum")))
        (bind _output_get (set `local.PossibleTiles` _shape_3))
        (return _output_get)
        (else
          (bind _result (`BlueprintSetLibrary.Set_ToArray` (`local.AvailableNeighbors`)))
          (set `local.PossibleTiles` _result)
          (return (`local.PossibleTiles`)))))))

(fn `GetUncontrolledTiles`
  (returns (ReturnValue :type "Array of IntPoint Structure"))
  (bind _shape (`self.Find Tiles Of Status` (`|MakeArray` "NotOwned" :!type "ETileStatus Enum")))
  (return _shape))

(fn `Hex_Logic_Definitions`
  (locals (Cube :type "IntVector Structure") (Axial :type "IntPoint Structure") (Offset :type "IntPoint Structure") (Polar :type "IntPoint Structure") (Location :type "Vector Structure") (Index :type Integer) (Steps :type Integer) (Degrees :type "Float (double-precision)") (Adjacent :type "/Game/ExternalContent/Hex_Grid_Toolkit/BluePrints/Hex_Logic/E_Hex_Dir_Adjacent Enum") (Diagonal :type "/Game/ExternalContent/Hex_Grid_Toolkit/BluePrints/Hex_Logic/E_Hex_Dir_Diagonal Enum") (Combined :type "/Game/ExternalContent/Hex_Grid_Toolkit/BluePrints/Hex_Logic/E_Hex_Dir_Combined Enum") (Shape :type "Array of IntPoint Structure") (Path :type "Array of IntPoint Structure") (TileActorMap :type "Map of IntPoint Structure to /Game/ExternalContent/Hex_Grid_Toolkit/BluePrints/Tile_Logic/BP_Tile Object Reference") (FlowMap :type "Map of IntPoint Structure to IntPoint Structure") (CostMap :type "Map of IntPoint Structure to Integer") (BP_Tile :type "/Game/ExternalContent/Hex_Grid_Toolkit/BluePrints/Tile_Logic/BP_Tile Object Reference"))
  ;[1 0.6667 0] Dictionary of key concepts and naming conventions . To understand this toolkit.
)

(fn `setTileSight`
  (params (Axial :type "Array of IntPoint Structure") (bSight :type Boolean))
  (for _array_element Axial
    (if (`.ReturnValue` (`BlueprintMapLibrary.Map_Find` (`self.Tiles`) _array_element))
      _)))

(fn `spawnTile`
  (params (Axial :type "IntPoint Structure"))
  (bind (_value _returnvalue) (`BlueprintMapLibrary.Map_Find` (`self.Tiles`) Axial))
  (`|ExecutionSequence`
    (:`then_0`
      ;[1 1 1] If actor exist at that axial, destroy it
      (if _returnvalue
        (`self.K2_DestroyActor` _value)))
    (:`then_1`
      (bind _returnvalue_2 (`|SpawnActorFromClass` "/Game/BattleMinds/Core/Tiles/BP_TileBase.BP_TileBase_C" (`KismetMathLibrary.MakeTransform` (0.0 0.0 0.0)) "Undefined" "OverrideRootScale" null Axial null))
      (`BlueprintMapLibrary.Map_Add` (`self.Tiles`) Axial _returnvalue_2))))

(fn `UserConstructionScript`)