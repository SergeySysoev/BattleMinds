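; Game mode for BattleMinds that sets up joining players and runs timed quiz questions.
; On login, each player state receives a material and nickname picked from map values by join order.
; OpenQuestion picks a random row from DT_Questions_Choose and has every player controller open its question widget.
; A timer then calls GatherPlayersAnswers, which currently only removes those widgets without collecting any answers.
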(event `self.K2_PostLogin`
  (params (NewPlayer :type "PlayerController Object Reference"))
  (`self.InitPlayer` NewPlayer)
  (`/Engine/EditorBlueprintResources/StandardMacros.IncrementInt` (`self.NumberOfPlayers`)))

(event `InitPlayer`
  (params (PlayerController :type "Controller Object Reference"))
  (bind _values (`BlueprintMapLibrary.Map_Values` (`self.MaterialMap`)))
  (bind _asbp_player_state (cast `/Game/BattleMinds/Core/Player/BP_PlayerState` (`Controller.PlayerState` PlayerController)))
  (set `BM_PlayerState.Material` (`|GetArrayItem` _values (`self.NumberOfPlayers`)) _asbp_player_state)
  (bind _values_2 (`BlueprintMapLibrary.Map_Values` (`self.Nicknames`)))
  (set `BM_PlayerState.Nickname` (`|GetArrayItem` _values_2 (`self.NumberOfPlayers`)) _asbp_player_state))

(event `OpenQuestion`
  (bind _outrownames (`DataTableFunctionLibrary.GetDataTableRowNames` "/Game/BattleMinds/Data/DT_Questions_Choose.DT_Questions_Choose"))
  (set `self.QuestionName` (`|GetArrayItem` _outrownames (`KismetMathLibrary.RandomIntegerInRange` 0 (- (`KismetArrayLibrary.Array_Length` _outrownames) 1))))
  (bind _asbp_game_state_classic (cast `/Game/BattleMinds/Core/GameStates/BP_GameStateClassic` (`GameplayStatics.GetGameState`)))
  (for _array_element (`GameStateBase.PlayerArray` _asbp_game_state_classic)
    (bind _asbp_player_controller (cast `/Game/BattleMinds/Core/Player/BP_PlayerController` (`PlayerState.GetPlayerController` _array_element)))
    (`KismetSystemLibrary.PrintString` (`KismetStringLibrary.Conv_NameToString` (`self.QuestionName`)))
    (`/Game/BattleMinds/Core/Player/BP_PlayerController.CC_OpenQuestionWidget` _asbp_player_controller (`self.QuestionName`)))
  (`self.StartQuestionTimer`))

(event `StartQuestionTimer`
  (bind _returnvalue (`KismetSystemLibrary.K2_SetTimerDelegate` (delegate `GatherPlayersAnswers`) (`self.QuestionTimer`)))
  (set `self.QuestionTimerHandle` _returnvalue))

(event `GatherPlayersAnswers`
  (bind _asbp_game_state_classic (cast `/Game/BattleMinds/Core/GameStates/BP_GameStateClassic` (`GameplayStatics.GetGameState`)))
  (for _array_element (`GameStateBase.PlayerArray` _asbp_game_state_classic)
    (bind _asbp_player_controller (cast `/Game/BattleMinds/Core/Player/BP_PlayerController` (`PlayerState.GetPlayerController` _array_element)))
    (`/Game/BattleMinds/Core/Player/BP_PlayerController.CC_RemoveQuestionWidget` _asbp_player_controller)))

(fn `UserConstructionScript`)