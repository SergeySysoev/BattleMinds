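; Lobby actor that spawns and manages preview models of a player's castle and banner.
; It spawns each preview at its own mesh point, owned by player controller 0, and tracks them in static and skeletal mesh actor arrays.
; SC-prefixed events recolor the tracked previews, together or by type, or destroy them all.
; It also stores an owning player controller as its own owner and can report whether one is valid.
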(event `self.ReceiveBeginPlay`)

(event `SetOwningPlayerController`
  (params (OwningPC :type "/Game/BattleMinds/Core/Lobby/BP_PC_Lobby Object Reference"))
  (bind _output_get (set `self.OwningPC` OwningPC))
  (`self.SetOwner` _output_get))

(event `SC_SpawnMeshes`
  (`self.SC_SpawnCastleMeshPreview`)
  (`self.SC_SpawnBannerMeshPreview`))

(event `SC_UpdateColor`
  (params (Color :type "EColor Enum" :default "Red"))
  ;[1 1 1] Visuals
  (`self.SC_UpdateColorOfCastle` Color)
  (`self.SC_UpdateColorOfBanner` Color))

(event `SC_UpdateColorOfCastle`
  (params (NewColor :type "EColor Enum" :default "Red"))
  ;[1 1 1] Visuals
  (for _array_element (`self.SpawnedStaticMeshActors`)
    (`/Engine/EditorBlueprintResources/StandardMacros.IsValid` _array_element
      (:`Is Valid`
        (`/Game/BattleMinds/Core/Lobby/BP_StaticMeshPreview.SC_UpdateColor` _array_element NewColor)))))

(event `SC_UpdateColorOfBanner`
  (params (NewColor :type "EColor Enum" :default "Red"))
  ;[1 1 1] Visuals
  (for _array_element (`self.SpawnedSkeletalMeshActors`)
    (`/Engine/EditorBlueprintResources/StandardMacros.IsValid` _array_element
      (:`Is Valid`
        (`/Game/BattleMinds/Core/Lobby/BP_SkeletalMeshPreview.SC_UpdateColor` _array_element NewColor)))))

(event `SC_SpawnCastleMeshPreview`
  ;[1 1 1] Visuals
  (bind _returnvalue (`|SpawnActorFromClass` "/Game/BattleMinds/Core/Lobby/BP_Castle_preview.BP_Castle_preview_C" (`KismetMathLibrary.MakeTransform` (`SceneComponent.K2_GetComponentLocation` (`self.CastleMeshPoint`))) "Undefined" "MultiplyWithRoot" (`GameplayStatics.GetPlayerController` 0) null))
  (`KismetArrayLibrary.Array_Add` (`self.SpawnedStaticMeshActors`) _returnvalue))

(event `SC_SpawnBannerMeshPreview`
  ;[1 1 1] Visuals
  (bind _returnvalue (`|SpawnActorFromClass` "/Game/BattleMinds/Core/Lobby/BP_Banner_Preview.BP_Banner_Preview_C" (`KismetMathLibrary.MakeTransform` (`SceneComponent.K2_GetComponentLocation` (`self.BannerMeshPoint`))) "Undefined" "MultiplyWithRoot" (`GameplayStatics.GetPlayerController` 0) null))
  (`KismetArrayLibrary.Array_Add` (`self.SpawnedSkeletalMeshActors`) _returnvalue))

(event `SC_DestroySpawnedActors`
  (for _array_element (`self.SpawnedStaticMeshActors`)
    (`self.K2_DestroyActor` _array_element))
  (for _array_element_2 (`self.SpawnedSkeletalMeshActors`)
    (`self.K2_DestroyActor` _array_element_2)))

(fn `Has Owning Controller`
  (returns (HasOwner :type Boolean))
  (return (`KismetSystemLibrary.IsValid` (`self.OwningPC`))))

(fn `UserConstructionScript`)