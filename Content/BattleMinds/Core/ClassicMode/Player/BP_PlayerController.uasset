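; Player controller for Classic Mode that handles hex-tile clicks and relays turn and question interactions.
; On begin play it adds the lobby input context locally and caches the tile manager; left-click traces to a tile and, unless attacked, sends its axial coordinate through a server call.
; Wrapper events route HUD turn, timer, round and border-blink updates through multicast and client calls.
; Debug events drive game state; older hover and selection logic is disconnected.
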(event `UpdateSelectedHex`
  ;[1 0 0] Debug Hex
  (bind _hextilemanager (`self.HexTileManager`)
    (:`then`
      (`/Game/ExternalContent/Hex_Grid_Toolkit/BluePrints/Tile_Logic/BP_Tile_Manager.HexSelectedUpdate` _hextilemanager))
    (:`else`)))

(event `UpdateHoveredHex`
  ;[1 0 0] Debug Hex
  (bind _hextilemanager (`self.HexTileManager`)
    (:`then`
      (`/Game/ExternalContent/Hex_Grid_Toolkit/BluePrints/Tile_Logic/BP_Tile_Manager.HexHoverUpdate` _hextilemanager))
    (:`else`)))

(event `self.ReceiveBeginPlay`
  (if (`self.IsLocalPlayerController`)
    (`EnhancedInputSubsystemInterface.AddMappingContext` (subsystem `EnhancedInputLocalPlayerSubsystem`) "/Game/BattleMinds/Input/IMC_Lobby.IMC_Lobby" 0 (struct))
    (bind _returnvalue (`GameplayStatics.GetActorOfClass` "/Game/ExternalContent/Hex_Grid_Toolkit/BluePrints/Tile_Logic/BP_Tile_Manager.BP_Tile_Manager_C"))
    (set `self.HexTileManager` _returnvalue)))

(event `Key|LeftMouseButton`
  (params (Key :type "Key Structure"))
  ;[1 1 1] Tile Conrol
  (:`Pressed`
    (bind _asbp_tile_base (cast `/Game/BattleMinds/Core/Tiles/BP_TileBase` (`.HitActor` (`GameplayStatics.BreakHitResult` (`self.GetHitResultUnderCursorForObjects` (`|MakeArray` "ObjectTypeQuery7" :!type "EObjectTypeQuery Enum"))))))
    (if (not (`BM_TileBase.bIsAttacked` _asbp_tile_base))
      (`self.SC_TryClickTheTile` (`BM_TileBase.GetAxial` _asbp_tile_base)))))

(event `self.ReceiveTick`
  (params (DeltaSeconds :type "Float (single-precision)")))

(event `self.OpenQuestion`
  ;[1 0.1394 0.6861] Widget Interactions
  (`self.SC_RequestToOpenQuestion` "Choose"))

(event `self.UpdateCurrentPlayerNickname`
  (params (CurrentPlayerID :type Integer))
  ;[1 0.1394 0.6861] Widget Interactions
  (`self.MC_UpdateCurrentPlayerNickname` CurrentPlayerID))

(event `MC_UpdateCurrentPlayerNickname`
  (params (PlayerID :type Integer))
  ;[1 0.1394 0.6861] Widget Interactions
  (bind _aswbp_player_hud (cast `/Game/BattleMinds/UI/HUD/WBP_PlayerHUD` (`self.PlayerHUD`)))
  (`/Game/BattleMinds/UI/HUD/WBP_PlayerHUD.UpdatePlayersTurn` _aswbp_player_hud PlayerID))

(event `self.ResetTurnTimer`
  (params (GameRound :type "EGameRound Enum" :default "ChooseCastle"))
  ;[1 0.1394 0.6861] Widget Interactions
  (`self.CC_ResetTurnTimer` GameRound))

(event `self.SetPlayerBorderBlinking`
  (params (IsEnabled :type Boolean))
  ;[1 0.1394 0.6861] Widget Interactions
  (`self.MC_SetPlayerBorderBlinking` IsEnabled))

(event `self.StartCountdownTimer`
  ;[1 0.1394 0.6861] Widget Interactions
  (`self.CC_StartTurnTImer`))

(event `MC_SetPlayerBorderBlinking`
  (params (IsEnabled :type Boolean))
  ;[1 0.1394 0.6861] Widget Interactions
  (bind _aswbp_player_hud (cast `/Game/BattleMinds/UI/HUD/WBP_PlayerHUD` (`self.PlayerHUD`)))
  (`/Game/BattleMinds/UI/HUD/WBP_PlayerHUD.SetPlayersBorderBlinking` _aswbp_player_hud IsEnabled))

(event `CC_StartTurnTImer`
  ;[1 0.1394 0.6861] Widget Interactions
  (bind _playerhud (`self.PlayerHUD`)
    (:`then`
      (bind _aswbp_player_hud (cast `/Game/BattleMinds/UI/HUD/WBP_PlayerHUD` _playerhud))
      (`/Game/BattleMinds/UI/HUD/WBP_PlayerHUD.StartTurnTimer` _aswbp_player_hud))
    (:`else`)))

(event `CC_ResetTurnTimer`
  (params (GameRound :type "EGameRound Enum" :default "ChooseCastle"))
  ;[1 0.1394 0.6861] Widget Interactions
  (bind _playerhud (`self.PlayerHUD`)
    (:`then`
      (bind _aswbp_player_hud (cast `/Game/BattleMinds/UI/HUD/WBP_PlayerHUD` _playerhud))
      (`/Game/BattleMinds/UI/HUD/WBP_PlayerHUD.StopTurnTimer` _aswbp_player_hud)
      (`/Game/BattleMinds/UI/HUD/WBP_GameRoundIndicator.SetRoundIndicator` (`/Game/BattleMinds/UI/HUD/WBP_PlayerHUD.WBP_GameRoundIndicator` _aswbp_player_hud) GameRound))
    (:`else`)))

(event `SC_CallStartGame`
  ;[1 0 0] Debug
  (bind _asbp_game_state_classic (cast `/Game/BattleMinds/Core/ClassicMode/Core/BP_GameStateClassic` (`GameplayStatics.GetGameState`)))
  (`BM_GameStateBase.StartPlayerTurnTimer` _asbp_game_state_classic 0))

(event `SC_SetGameRound`
  (params (NewRound :type "EGameRound Enum" :default "ChooseCastle"))
  ;[1 0 0] Debug
  (bind _asbp_game_state_classic (cast `/Game/BattleMinds/Core/ClassicMode/Core/BP_GameStateClassic` (`GameplayStatics.GetGameState`)))
  (`BM_GameStateClassic.ForceSetGameRound` _asbp_game_state_classic NewRound))

(fn `UserConstructionScript`)