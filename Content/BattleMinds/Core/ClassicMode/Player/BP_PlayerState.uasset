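; BP_PlayerState is the Classic Mode player state, tracking a player's answered quiz questions and points.
; SC_AddAnsweredQuestion flags the current answer as sent, stores the question, and prints debug results by type: correctness flag for Choose Answer, exact answer and elapsed time for Shot.
; SetPointsinWidget pushes Points to the HUD through the player controller returned by GetPlayerController.
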(event `self.ReceiveBeginPlay`)

(event `SC_AddAnsweredQuestion`
  (params (Question :type "Question Structure"))
  (bind (_question _type _answers _answershot _pointsmodifier _bwasanswered _playerid _bexactanswer _elapsedtime) (break `Question` Question))
  (bind (_days _hours _minutes _seconds _milliseconds) (`KismetMathLibrary.BreakTimespan` _elapsedtime))
  (set `self.CurrentQuestionAnswerSent` true)
  (`KismetArrayLibrary.Array_Add` (`self.AnsweredQuestions`) Question)
  (switch `EQuestionType` _type
    (:`Choose`
      (`KismetSystemLibrary.PrintString` (`KismetStringLibrary.Conv_BoolToString` _bwasanswered)))
    (:`Shot`
      (`KismetSystemLibrary.PrintString` (`KismetStringLibrary.Concat_StrStr` (`KismetStringLibrary.Conv_BoolToString` _bexactanswer) ", Time:    " (`KismetStringLibrary.Conv_IntToString` _seconds) ":" (`KismetStringLibrary.Conv_IntToString` _milliseconds))))))

(event `self.SetPointsInWidget`
  (bind _asbp_player_controller (cast `/Game/BattleMinds/Core/ClassicMode/Player/BP_PlayerController` (`self.GetPlayerController`)))
  (`/Game/BattleMinds/Core/UI/WBP_PlayerInfo.SetPoints` (`/Game/BattleMinds/Core/ClassicMode/Player/BP_PlayerController.PlayerHUD` _asbp_player_controller) (`self.Points`)))

(fn `UserConstructionScript`)