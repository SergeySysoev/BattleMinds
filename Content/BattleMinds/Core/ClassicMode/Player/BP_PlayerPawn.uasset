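; Player camera pawn for BattleMinds Classic Mode that moves the view between an above-map player-turn position and a default position behind the player's castle.
; TravelCamera runs movement-locked, curve-driven Universal Camera travels, snapping to the target if aborted and skipping travel when already there.
; The player-turn branch then calls CallCheckPrePlayerTurnPhaseHandled on arrival, abort or skip.
; Enhanced Input actions drive zoom and yaw rotation around a pivot.
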(event `self.ReceiveBeginPlay`)

(event `self.TravelCamera`
  (params (IsPlayerTurn :type Boolean))
  (bind _playerturncameraproperties (`self.PlayerTurnCameraProperties`))
  (bind _defaultcameraproperties (`self.DefaultCameraProperties`))
  (bind _defaultcameraproperties_2 (`self.DefaultCameraProperties`))
  (bind _playerturncameraproperties_2 (`self.PlayerTurnCameraProperties`))
  (if (`self.IsTraveling`)
    (`self.AbortTravelTask`))
  (if IsPlayerTurn
    ;[1 1 1] Player Turn Camera above the map
    (if (not (== (`self.DesiredLocation`) (`.DesiredLocation` (break `UniversalCameraPositionSaveFormat` (`self.PlayerTurnCameraProperties`))) :`ErrorTolerance` 0.001))
      (`AsyncNode.CameraTravel` self (struct) (`AsyncNode.UseCustomLocation` (break `UniversalCameraPositionSaveFormat` _playerturncameraproperties)) (struct) (`AsyncNode.UseCustomValue` (.yaw (`.DesiredRotation` (break `UniversalCameraPositionSaveFormat` _playerturncameraproperties)))) (`AsyncNode.UseCustomValue` (.pitch (`.DesiredRotation` (break `UniversalCameraPositionSaveFormat` _playerturncameraproperties)))) (`AsyncNode.UseCustomValue` (.roll (`.DesiredRotation` (break `UniversalCameraPositionSaveFormat` _playerturncameraproperties)))) (`AsyncNode.UseCustomValue` (`.DesiredZoom` (break `UniversalCameraPositionSaveFormat` _playerturncameraproperties))) "/Game/BattleMinds/Developer/Curve_CameraTravel.Curve_CameraTravel" (struct) true
        (:`OnReachedDestination`
          _)
        (:`OnAborted`
          (`self.SetDesiredPosition` (break `UniversalCameraPositionSaveFormat` _playerturncameraproperties_2) (`.DesiredTargetOffset` (break `UniversalCameraPositionSaveFormat` _playerturncameraproperties_2)) (`.DesiredSocketOffset` (break `UniversalCameraPositionSaveFormat` _playerturncameraproperties_2)) (.yaw (`.DesiredRotation` (break `UniversalCameraPositionSaveFormat` _playerturncameraproperties_2))) (.pitch (`.DesiredRotation` (break `UniversalCameraPositionSaveFormat` _playerturncameraproperties_2))) (.roll (`.DesiredRotation` (break `UniversalCameraPositionSaveFormat` _playerturncameraproperties_2))) (`.DesiredZoom` (break `UniversalCameraPositionSaveFormat` _playerturncameraproperties_2)) false true))))
    (`self.CallCheckPrePlayerTurnPhaseHandled`)
    (elif (not (== (`self.DesiredLocation`) (`.DesiredLocation` (break `UniversalCameraPositionSaveFormat` (`self.DefaultCameraProperties`))) :`ErrorTolerance` 0.001))
      ;[1 1 1] Castle Camera behind the Player Castle
      (`AsyncNode.CameraTravel` self (struct) (`AsyncNode.UseCustomLocation` (break `UniversalCameraPositionSaveFormat` _defaultcameraproperties)) (struct) (`AsyncNode.UseCustomValue` (.yaw (`.DesiredRotation` (break `UniversalCameraPositionSaveFormat` _defaultcameraproperties)))) (`AsyncNode.UseCustomValue` (.pitch (`.DesiredRotation` (break `UniversalCameraPositionSaveFormat` _defaultcameraproperties)))) (`AsyncNode.UseCustomValue` (.roll (`.DesiredRotation` (break `UniversalCameraPositionSaveFormat` _defaultcameraproperties)))) (`AsyncNode.UseCustomValue` (`.DesiredZoom` (break `UniversalCameraPositionSaveFormat` _defaultcameraproperties))) "/Game/BattleMinds/Developer/Curve_CameraTravel.Curve_CameraTravel" (struct) true
        (:`OnAborted`
          (`self.SetDesiredPosition` (break `UniversalCameraPositionSaveFormat` _defaultcameraproperties_2) (`.DesiredTargetOffset` (break `UniversalCameraPositionSaveFormat` _defaultcameraproperties_2)) (`.DesiredSocketOffset` (break `UniversalCameraPositionSaveFormat` _defaultcameraproperties_2)) (.yaw (`.DesiredRotation` (break `UniversalCameraPositionSaveFormat` _defaultcameraproperties_2))) (.pitch (`.DesiredRotation` (break `UniversalCameraPositionSaveFormat` _defaultcameraproperties_2))) (.roll (`.DesiredRotation` (break `UniversalCameraPositionSaveFormat` _defaultcameraproperties_2))) (`.DesiredZoom` (break `UniversalCameraPositionSaveFormat` _defaultcameraproperties_2)) false true))))))

(event `EnhancedInput|/Game/BattleMinds/Input/IA_CameraZoom`
  (params (ActionValue :type "Float (double-precision)") (ElapsedSeconds :type "Float (double-precision)") (TriggeredSeconds :type "Float (double-precision)") (InputAction :type "InputAction Object Reference" :default "/Game/BattleMinds/Input/IA_CameraZoom.IA_CameraZoom"))
  ;[1 1 1] Inputs
  (:`Triggered`
    (`self.ZoomIn` ActionValue)))

(event `EnhancedInput|/Game/BattleMinds/Developer/IA_RotateYaw`
  (params (ActionValue :type "Float (double-precision)") (ElapsedSeconds :type "Float (double-precision)") (TriggeredSeconds :type "Float (double-precision)") (InputAction :type "InputAction Object Reference" :default "/Game/BattleMinds/Developer/IA_RotateYaw.IA_RotateYaw"))
  ;[1 1 1] Inputs
  (:`Triggered`
    (`self.RotateYawAroundPivot` (`self.RotationPivotLocation`) ActionValue)))

(fn `UserConstructionScript`)