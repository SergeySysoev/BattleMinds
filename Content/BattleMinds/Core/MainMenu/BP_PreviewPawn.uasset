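; BP_PreviewPawn is a main-menu character that acts out attack and defence previews with sword-and-shield, twin swords or bow.
; PrepareForPreview turns it toward a target, then either equips and plays the chosen weapon's attack montage or readies sword-and-shield with a weighted random evade roll.
; ShotArrow spawns a preview projectile, while hit events play a block or death-and-recovery sequence.
; Construction toggles weapon mesh visibility and applies the color-mapped material.
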(event `PrepareForPreview`
  (params (RotationTarget :type "Actor Object Reference") (NewWeapon :type "/Game/BattleMinds/Core/MainMenu/E_WeaponPreviewType Enum" :default "NewEnumerator0") (State :type "/Game/BattleMinds/Core/MainMenu/E_PreviewState Enum" :default "NewEnumerator0"))
  (`SkeletalMeshComponent.Stop` (`self.SkeletalMesh`))
  (`|ExecutionSequence`
    (:`then_0`
      (bind _output_get (set `self.State` State))
      (if (`|EnumEquality` _output_get "NewEnumerator1")
        (`self.SwitchWeapon` NewWeapon)
        (else
          (set `self.EvadeDeath` (`KismetMathLibrary.RandomBoolWithWeight` 0.7))
          (`self.SwitchWeapon` "NewEnumerator0"))))
    (:`then_1`
      (`self.RotateToTarget` RotationTarget)
      (`self.PlayCorrespondingAnimation`))))

(event `PlayCorrespondingAnimation`
  (if (`|EnumEquality` (`self.State`) "NewEnumerator1")
    (`|PlayMontage` (`self.SkeletalMesh`) (select `/Game/BattleMinds/Core/MainMenu/E_WeaponPreviewType` (`self.CurrentWeapon`) :`NewEnumerator0` "/Game/ExternalContent/ModularRPGHeroesPolyart/Animations/SwordAndShieldStance/AM_Combo01_SwordShield.AM_Combo01_SwordShield" :`NewEnumerator1` "/Game/ExternalContent/ModularRPGHeroesPolyart/Animations/DoubleSwordStance/AM_Combo01_DoubleSword.AM_Combo01_DoubleSword" :`NewEnumerator2` "/Game/ExternalContent/ModularRPGHeroesPolyart/Animations/BowStance/AM_Attack01_Bow.AM_Attack01_Bow" :!type "AnimMontage Object Reference")
      (:`OnCompleted`
        (`self.SwitchWeapon` "NewEnumerator0")
        (set `self.State` "NewEnumerator0")))))

(event `ShotArrow`
  (bind _returnvalue (`|SpawnActorFromClass` "/Game/BattleMinds/Core/MainMenu/BP_PreviewArrowProjectile.BP_PreviewArrowProjectile_C" (`SceneComponent.GetSocketTransform` (`self.SkeletalMesh`) "RightWeaponShield" "RTS_World") "AlwaysSpawn" "MultiplyWithRoot" self self))
  (set `self.SpawnedArrow` _returnvalue))

(event `EditorPreviewAttackAnimation`)

(event `/Game/BattleMinds/Core/MainMenu/BPI_PreviewCombat.OnArrowHit`
  (`self.ReactToHit`))

(event `ReactToHit`
  (`|PlayMontage` (`self.SkeletalMesh`) (select `bool` (`self.EvadeDeath`) :`false` "/Game/ExternalContent/ModularRPGHeroesPolyart/Animations/SwordAndShieldStance/AM_Die_SwordShield.AM_Die_SwordShield" :`true` "/Game/ExternalContent/ModularRPGHeroesPolyart/Animations/SwordAndShieldStance/AM_DefendHit_SwordShield.AM_DefendHit_SwordShield" :!type "AnimMontage Object Reference")
    (:`OnBlendOut`
      (if (`self.EvadeDeath`)
        (set `self.State` "NewEnumerator0")
        (else
          (set `self.State` "NewEnumerator3")
          (`KismetSystemLibrary.Delay` 1.0)
          (`self.RecoverAfterHit`))))))

(event `RecoverAfterHit`
  (`|PlayMontage` (`self.SkeletalMesh`) "/Game/ExternalContent/ModularRPGHeroesPolyart/Animations/SwordAndShieldStance/AM_DieRecover_SwordShield.AM_DieRecover_SwordShield"
    (:`OnBlendOut`
      (set `self.State` "NewEnumerator0"))))

(fn `RotateToTarget`
  (params (Target :type "Actor Object Reference"))
  (bind (_returnvalue_roll _returnvalue_pitch _returnvalue_yaw) (`KismetMathLibrary.BreakRotator` (`KismetMathLibrary.FindLookAtRotation` (`self.K2_GetActorLocation`) (`self.K2_GetActorLocation` Target))))
  (`self.K2_SetActorRotation` (`KismetMathLibrary.MakeRotator` 0.0 0.0 _returnvalue_yaw)))

(fn `SetWeaponVisibility`
  (params (bVisible :type Boolean))
  (switch `/Game/BattleMinds/Core/MainMenu/E_WeaponPreviewType` (`self.CurrentWeapon`)
    (:`NewEnumerator0`
      (`SceneComponent.SetVisibility` (`self.Shield`) (`local.bVisible`) false)
      (`SceneComponent.SetVisibility` (`self.RightWeapon`) (`local.bVisible`) false))
    (:`NewEnumerator1`
      (`SceneComponent.SetVisibility` (`self.RightWeapon`) (`local.bVisible`) false)
      (`SceneComponent.SetVisibility` (`self.LeftWeapon`) (`local.bVisible`) false))
    (:`NewEnumerator2`
      (`SceneComponent.SetVisibility` (`self.Bow`) (`local.bVisible`) false)
      (`SceneComponent.SetVisibility` (`self.Arrow`) (`local.bVisible`) false))))

(fn `SwitchMaterial`
  (bind _skeletalmesh (`self.SkeletalMesh`))
  (bind (_value _returnvalue) (`BlueprintMapLibrary.Map_Find` (`self.Materials`) (`self.Color`)))
  (if _returnvalue
    (`PrimitiveComponent.SetMaterial` _skeletalmesh 0 _value)
    (`PrimitiveComponent.SetMaterial` (`self.Arrow`) 0 _value)
    (`PrimitiveComponent.SetMaterial` (`self.Bow`) 0 _value)
    (`PrimitiveComponent.SetMaterial` (`self.RightWeapon`) 0 _value)
    (`PrimitiveComponent.SetMaterial` (`self.Shield`) 0 _value)
    (`PrimitiveComponent.SetMaterial` (`self.LeftWeapon`) 0 _value)
    (else
      (`PrimitiveComponent.SetMaterial` _skeletalmesh 0 "/Game/ExternalContent/ModularRPGHeroesPolyart/Materials/PolyartMat.PolyartMat")
      (`PrimitiveComponent.SetMaterial` (`self.Arrow`) 0 "/Game/ExternalContent/ModularRPGHeroesPolyart/Materials/PolyartMat.PolyartMat")
      (`PrimitiveComponent.SetMaterial` (`self.Bow`) 0 "/Game/ExternalContent/ModularRPGHeroesPolyart/Materials/PolyartMat.PolyartMat")
      (`PrimitiveComponent.SetMaterial` (`self.RightWeapon`) 0 "/Game/ExternalContent/ModularRPGHeroesPolyart/Materials/PolyartMat.PolyartMat")
      (`PrimitiveComponent.SetMaterial` (`self.Shield`) 0 "/Game/ExternalContent/ModularRPGHeroesPolyart/Materials/PolyartMat.PolyartMat")
      (`PrimitiveComponent.SetMaterial` (`self.LeftWeapon`) 0 "/Game/ExternalContent/ModularRPGHeroesPolyart/Materials/PolyartMat.PolyartMat"))))

(fn `SwitchWeapon`
  (params (NewWeapon :type "/Game/BattleMinds/Core/MainMenu/E_WeaponPreviewType Enum" :default "NewEnumerator0"))
  (`self.SetWeaponVisibility` false)
  (set `self.CurrentWeapon` NewWeapon)
  (`self.SetWeaponVisibility` true))

(fn `UserConstructionScript`
  (`self.SwitchWeapon` (`self.CurrentWeapon`))
  (`self.SwitchMaterial`))