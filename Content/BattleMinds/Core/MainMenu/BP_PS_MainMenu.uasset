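; Player state for the main menu that sets up the local player's Steam identity.
; On BeginPlay, it requests the small Steam avatar for the player controller's unique net ID.
; On success, it stores the Steam persona name and avatar as the player's nickname and avatar.
; On failure, it falls back to a debug nickname and a placeholder avatar texture.
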(event `self.ReceiveBeginPlay`
  (`parent.ReceiveBeginPlay`)
  (`self.InitPlayerSteamInfo`))

(event `InitPlayerSteamInfo`
  (bind _uniquenetid (`AdvancedSessionsLibrary.GetUniqueNetID` (`self.GetPlayerController`)))
  (bind _returnvalue (`AdvancedSteamFriendsLibrary.GetSteamFriendAvatar` _uniquenetid "SteamAvatar_Small")
    (:`OnSuccess`
      (bind _returnvalue_2 (`AdvancedSteamFriendsLibrary.GetSteamPersonaName` _uniquenetid))
      (`self.SetPlayerNickname` _returnvalue_2)
      (`self.SetPlayerAvatar` _returnvalue))
    (:`OnFailure`
      (`self.SetPlayerNickname` "DebugPlayer")
      (`self.SetPlayerAvatar` "/Game/BattleMinds/Assets/Widgets/Profile_Pics/T_Avatar_Image_1.T_Avatar_Image_1"))))

(fn `UserConstructionScript`)