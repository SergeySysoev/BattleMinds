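; Player controller for a tile-based game that creates the local player's info HUD and handles tile clicks.
; Left click traces under the cursor for a BM_TileBase and passes it to SCTryClickTheTile, which is not defined here.
; A separate SC-to-MC ChangeTile event chain applies the PlayerState's material and this controller as owner to a tile.
; The only SCChangeTile call in this graph is disconnected.
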(event `self.ReceiveBeginPlay`
  (if (`self.IsLocalPlayerController`)
    (bind _returnvalue (`|CreateWidget` "/Game/UI/WBP_PlayerInfo.WBP_PlayerInfo_C" self))
    (`UserWidget.AddToViewport` _returnvalue 0)))

(event `Key|LeftMouseButton`
  (params (Key :type "Key Structure"))
  (bind (_asbm_tile_base _bsuccess) (cast `BM_TileBase` (`.HitActor` (`GameplayStatics.BreakHitResult` (`self.GetHitResultUnderCursorForObjects` (`|MakeArray` "ObjectTypeQuery7" :!type "EObjectTypeQuery Enum")))) :!pure true))
  (:`Pressed`
    (if _bsuccess
      (`self.SC_TryClickTheTile` _asbm_tile_base))))

(event `SC_ChangeTile`
  (params (Tile :type "/Game/Tiles/BP_TileBase Object Reference"))
  (`self.MC_ChangeTile` Tile))

(event `MC_ChangeTile`
  (params (Tile :type "/Game/Tiles/BP_TileBase Object Reference"))
  (`/Game/Tiles/BP_TileBase.SetMaterials` Tile (`BM_PlayerState.Material` (cast `/Game/Player/BP_PlayerState` (`self.PlayerState`) :!pure true)) self))

(fn `UserConstructionScript`)