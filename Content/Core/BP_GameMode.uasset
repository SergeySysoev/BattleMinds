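; Game mode that gives each joining player a material and a nickname.
; On PostLogin, InitPlayer casts the controller's PlayerState to BP_PlayerState and writes both values, taken from the MaterialMap and Nicknames map values at the current Players index.
; The Players counter then increments, so assignment follows join order, with no wraparound or bounds check on the index.
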(event `self.K2_PostLogin`
  (params (NewPlayer :type "PlayerController Object Reference"))
  (`self.InitPlayer` NewPlayer)
  (`/Engine/EditorBlueprintResources/StandardMacros.IncrementInt` (`self.Players`)))

(event `InitPlayer`
  (params (PlayerController :type "Controller Object Reference"))
  (bind _values (`BlueprintMapLibrary.Map_Values` (`self.MaterialMap`)))
  (bind _asbp_player_state (cast `/Game/Player/BP_PlayerState` (`Controller.PlayerState` PlayerController)))
  (set `BM_PlayerState.Material` (`|GetArrayItem` _values (`self.Players`)) _asbp_player_state)
  (bind _values_2 (`BlueprintMapLibrary.Map_Values` (`self.Nicknames`)))
  (set `BM_PlayerState.Nickname` (`|GetArrayItem` _values_2 (`self.Players`)) _asbp_player_state))

(fn `UserConstructionScript`)