(fn `Create_Notification`
  (params (Notification_Title :type Text) (Notification_Description :type Text) (Notification_Type :type "/Game/PopUp_System/Blueprints/E_Pop-up_Type Enum" :default "NewEnumerator0") (Duration :type "Float (single-precision)"))
  (if (`Controller.IsLocalPlayerController` (`GameplayStatics.GetPlayerController` null))
    (bind _foundwidgets (`WidgetBlueprintLibrary.GetAllWidgetsWithInterface` null "/Game/PopUp_System/Blueprints/BPI_Notifications.BPI_Notifications_C"))
    (message `/Game/PopUp_System/Blueprints/BPI_Notifications.Add_Notification` (`|GetArrayItem` _foundwidgets) Notification_Title Notification_Description Notification_Type Duration)))

(fn `Create_PopUp_1`
  (params (`Pop-up_Title` :type Text) (`Pop-up_Description` :type Text) (Left_Button_Text :type Text) (Right_Button_Text :type Text) (`Pop-up_Type` :type "/Game/PopUp_System/Blueprints/E_Pop-up_Type Enum" :default "NewEnumerator0"))
  (returns (Widget_Ref :type "/Game/PopUp_System/Widgets/WB_Pop-up_1 Object Reference"))
  (bind _returnvalue (`GameplayStatics.GetPlayerController` null))
  (if (`Controller.IsLocalPlayerController` _returnvalue)
    (bind _returnvalue_2 (`|CreateWidget` "/Game/PopUp_System/Widgets/WB_Pop-up_1.WB_Pop-up_1_C" _returnvalue `Pop-up_Title` `Pop-up_Description` Left_Button_Text Right_Button_Text `Pop-up_Type`))
    (`UserWidget.AddToViewport` _returnvalue_2 0)
    (return _returnvalue_2)))

(fn `Create_PopUp_2`
  (params (`Pop-up_Title` :type Text) (`Pop-up_Description` :type Text) (Left_Button_Text :type Text) (Right_Button_Text :type Text) (`Pop-up_Type` :type "/Game/PopUp_System/Blueprints/E_Pop-up_Type Enum" :default "NewEnumerator0"))
  (returns (Widget_Ref :type "/Game/PopUp_System/Widgets/WB_Pop-up_2 Object Reference"))
  (bind _returnvalue (`GameplayStatics.GetPlayerController` null))
  (if (`Controller.IsLocalPlayerController` _returnvalue)
    (bind _returnvalue_2 (`|CreateWidget` "/Game/PopUp_System/Widgets/WB_Pop-up_2.WB_Pop-up_2_C" _returnvalue `Pop-up_Title` `Pop-up_Description` Left_Button_Text Right_Button_Text `Pop-up_Type`))
    (`UserWidget.AddToViewport` _returnvalue_2 0)
    (return _returnvalue_2)))

(fn `Create_PopUp_3`
  (params (`Pop-up_Title` :type Text) (`Pop-up_Description` :type Text) (Left_Button_Text :type Text) (Right_Button_Text :type Text) (`Pop-up_Type` :type "/Game/PopUp_System/Blueprints/E_Pop-up_Type Enum" :default "NewEnumerator0"))
  (returns (Widget_Ref :type "/Game/PopUp_System/Widgets/WB_Pop-up_3 Object Reference"))
  (bind _returnvalue (`GameplayStatics.GetPlayerController` null))
  (if (`Controller.IsLocalPlayerController` _returnvalue)
    (bind _returnvalue_2 (`|CreateWidget` "/Game/PopUp_System/Widgets/WB_Pop-up_3.WB_Pop-up_3_C" _returnvalue `Pop-up_Title` `Pop-up_Description` Left_Button_Text Right_Button_Text `Pop-up_Type`))
    (`UserWidget.AddToViewport` _returnvalue_2 0)
    (return _returnvalue_2)))

(fn `Create_PopUp_4`
  (params (`Pop-up_Title` :type Text) (`Pop-up_Description` :type Text) (Left_Button_Text :type Text) (Right_Button_Text :type Text) (`Pop-up_Type` :type "/Game/PopUp_System/Blueprints/E_Pop-up_Type Enum" :default "NewEnumerator0"))
  (returns (Widget_Ref :type "/Game/PopUp_System/Widgets/WB_Pop-up_4 Object Reference"))
  (bind _returnvalue (`GameplayStatics.GetPlayerController` null))
  (if (`Controller.IsLocalPlayerController` _returnvalue)
    (bind _returnvalue_2 (`|CreateWidget` "/Game/PopUp_System/Widgets/WB_Pop-up_4.WB_Pop-up_4_C" _returnvalue `Pop-up_Title` `Pop-up_Description` Left_Button_Text Right_Button_Text `Pop-up_Type`))
    (`UserWidget.AddToViewport` _returnvalue_2 0)
    (return _returnvalue_2)))